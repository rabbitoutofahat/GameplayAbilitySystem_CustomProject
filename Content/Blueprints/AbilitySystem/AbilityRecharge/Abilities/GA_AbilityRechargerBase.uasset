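; Base Gameplay Ability for ability recharging, currently a debug skeleton that only watches the avatar's charge.
; On activation it starts a repeating attribute-change task on CurrentCharge and prints each new value.
; A next-tick check against MaxCharge that would cancel the ability at full charge is unwired, as is EndAbility, so nothing here recharges or ends it.
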(event Ability|EventActivateAbility
  (bind _newvalue (Ability|Tasks|WaitForAttributeChanged (Ability|GetAvatarActorfromActorInfo) (Variables|Default|GetCurrentCharge))
    (:Changed
      (Development|PrintString (Utilities|String|ToString(Float) _newvalue)))))