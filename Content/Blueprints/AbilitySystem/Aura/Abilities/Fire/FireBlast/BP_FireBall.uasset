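; BP_FireBall is the Fire Blast projectile, which flies out along its forward vector and then returns to its ReturnToActor.
; StartOutgoingTimeline runs only on authority, lerping the location out to an apex at TravelDistance through a timeline.
; A second timeline then lerps it back toward the target actor's live location.
; Once within ExplodeDistance on the return, it plays impact effects and destroys itself.
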(event EventStartOutgoingTimeline
  (Networking|SwitchHasAuthority
    (:Authority
      ;[1 0.8996 0.175] Store Initial and Apex Location Vectors
      (bind _output_get (Variables|Default|SetInitialLocation (Transformation|GetActorLocation)))
      (Variables|Default|SetApexLocation (+ _output_get (* (Transformation|GetActorForwardVector) (Variables|Default|GetTravelDistance))))
      (bind _outgoingtrack (Timeline|OutgoingTimeline Play)
        (:Update
          (Transformation|SetActorLocation (Math|Vector|Lerp(Vector) (Variables|Default|GetInitialLocation) (Variables|Default|GetApexLocation) _outgoingtrack) false false))
        (:Finished
          (bind _returningtrack (Timeline|ReturningTimeline Play)
            (:Update
              (Transformation|SetActorLocation (Math|Vector|Lerp(Vector) (Variables|Default|GetApexLocation) (Transformation|GetActorLocation (Variables|Default|GetReturnToActor)) _returningtrack) false false)
              (if (CallFunction|IsWithinExplodeDistance)
                (Class|AuraProjectile|PlayImpactEffects)
                (Actor|DestroyActor)))))))))

(fn ConstructionScript)

(fn IsWithinExplodeDistance
  (return (<= (Math|Vector|VectorLength (- (Transformation|GetActorLocation) (Transformation|GetActorLocation (Variables|Default|GetReturnToActor)))) (Variables|Default|GetExplodeDistance))))