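; Gameplay ability for enemy and summon melee attacks that faces the combat target and plays a random tagged attack montage.
; On the montage's gameplay event, it finds live players within attack radius of the tagged combat socket and damages those on other teams.
; A hit fires a replicated impact Gameplay Cue and grants summon avatars energy through a SetByCaller effect.
; The ability ends after the hit check or when the montage finishes.
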(event Ability|EventActivateAbility
  (Variables|Default|SetHasHitTarget false)
  (bind _output_get (Variables|Default|SetAvatarActor (Ability|GetAvatarActorfromActorInfo)))
  (bind _returnvalue (Class|CombatInterface|GetCombatTarget(Message) _output_get))
  (Class|CombatInterface|UpdateFacingTarget(Message) (Variables|Default|GetAvatarActor) (Transformation|GetActorLocation _returnvalue))
  (bind _returnvalue_2 (Class|CombatInterface|GetAttackMontages(Message) (Variables|Default|GetAvatarActor)))
  (bind _output_get_2 (Variables|Default|SetTaggedMontage (Class|AuraDamageGameplayAbility|GetRandomTaggedMontagefromArray _returnvalue_2)))
  (|PlayMontageandWaitProxy "None" (.Montage (Utilities|Struct|BreakTaggedMontage _output_get_2)) 1.0 "None" false 1.0 0.0 false
    (:then
      (Ability|Tasks|WaitGameplayEvent (.MontageTag (Utilities|Struct|BreakTaggedMontage _output_get_2)) 0
        (:EventReceived
          (bind _returnvalue_3 (Class|CombatInterface|GetCombatSocketLocation(Message) (Variables|Default|GetAvatarActor) (.SocketTag (Utilities|Struct|BreakTaggedMontage _output_get_2))))
          (bind _returnvalue_4 (Class|CombatInterface|GetAttackRadius(Message) (Variables|Default|GetAvatarActor)))
          (bind _output_get_3 (Variables|Default|SetCombatSocketLocation _returnvalue_3))
          (bind _outoverlappingactors (Class|AuraAbilitySystemLibrary|GetLivePlayersWithinRadius (Variables|Default|GetAvatarActor) (Utilities|Array|MakeArray (Variables|Default|GetAvatarActor)) _returnvalue_4 _output_get_3))
          (for _array_element _outoverlappingactors
            (if (not (Class|AuraAbilitySystemLibrary|IsonSameTeam _array_element (Variables|Default|GetAvatarActor)))
              (Class|AuraAbilitySystemLibrary|ApplyDamageEffecttoTarget (Class|AuraDamageGameplayAbility|MakeDamageEffectParamsfromClassDefaults _array_element))
              (Variables|Default|SetHasHitTarget true)
              (Class|CombatInterface|GetBloodEffect(Message) _array_element)))
          (if (Variables|Default|GetHasHitTarget)
            (CallFunction|ExecuteMeleeImpactCue)
            (bind _assummon_character (Utilities|Casting|CastToSummonCharacter (Variables|Default|GetAvatarActor))
              (:then
                (CallFunction|GrantEnergytoSummononHit _assummon_character))
              (:CastFailed
                _)))
          (Ability|EndAbility))))
    (:OnCompleted
      (Ability|EndAbility :!label _label))
    (:OnInterrupted
      (goto _label))
    (:OnCancelled
      (goto _label))))

(fn ExecuteMeleeImpactCue
  (bind _returnvalue (Class|CombatInterface|GetCombatTarget(Message) (Variables|Default|GetAvatarActor)))
  (Class|GameplayAbility|ExecuteGameplayCuewithParams "(TagName=\"GameplayCue.MeleeImpact\")" (Ability|GameplayCue|MakeGameplayCueParameters :AggregatedSourceTags (GameplayTags|MakeGameplayTagContainerfromTag (.MontageTag (Utilities|Struct|BreakTaggedMontage (Variables|Default|GetTaggedMontage)))) :Location (Variables|Default|GetCombatSocketLocation) :EffectCauser (Variables|Default|GetAvatarActor) :SourceObject _returnvalue)))

(fn GrantEnergytoSummononHit
  (params (SummonCharacter :type Summon%20Character%20Object%20Reference))
  (LocalVariables|SetAvatarASC (Ability|GetAbilitySystemComponent (Variables|Default|GetAvatarActor)))
  (bind _returnvalue (Class|CombatInterface|GetPlayerLevel(Message) (Variables|Default|GetAvatarActor)))
  (bind _returnvalue_2 (Ability|GameplayEffect|AssignTagSetbyCallerMagnitude (Ability|MakeOutgoingGameplayEffectSpec "/Game/Blueprints/AbilitySystem/Vessel/Effects/GE_EnergyRegen.GE_EnergyRegen_C" (Math|Conversions|ToFloat(Integer) _returnvalue)) (Variables|Default|GetEnergyTag) (Variables|/Script/Aura.SummonCharacter|GetEnergyOnHit SummonCharacter)))
  (GameplayEffects|ApplyGameplayEffectSpecToSelf (LocalVariables|GetAvatarASC) _returnvalue_2))