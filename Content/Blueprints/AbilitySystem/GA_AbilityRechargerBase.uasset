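; Base Gameplay Ability for recharging, which reacts to changes in the avatar's CurrentCharge attribute.
; On activation it starts a repeating attribute-change listener, then waits one tick after a change before comparing the new value with MaxCharge.
; Below max it prints a placeholder "Apply Recharge Effect" message and ends the ability, otherwise it cancels.
; No recharge effect is actually applied in this graph.
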(event Ability|EventActivateAbility
  (bind _returnvalue (Ability|GetAvatarActorfromActorInfo))
  (bind _newvalue (Ability|Tasks|WaitForAttributeChanged _returnvalue (Variables|Default|GetCurrentCharge))
    (:Changed
      (Utilities|FlowControl|DelayUntilNextTick)
      (if (< _newvalue (.ReturnValue (Ability|Attribute|GetFloatAttribute _returnvalue (Variables|Default|GetMaxCharge))))
        (Development|PrintString "Apply Recharge Effect")
        (Ability|EndAbility)
        (else
          (Ability|CancelAbility))))))