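; Demonfire Rift actor for a Vessel ability that periodically fires projectiles at random nearby enemies.
; On BeginPlay it gathers nearby enemies once and starts a looping timer that spreads the projectile count evenly across the spawn duration.
; Each tick of that timer spawns a projectile at a random target from the cached enemies.
; A separate duration timer is also set, and DestroyRift clears the spawn timer and destroys the actor.
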(event Custom|DestroyRift
  (Utilities|Time|ClearandInvalidateTimerbyHandle (Variables|Default|GetProjectileSpawnTimer))
  (Actor|DestroyActor))

(event Custom|ProjectileSpawn
  (Class|ProjectileSpawner|SpawnProjectileatRandomTarget (stale EventBeginPlay _returnvalue)))

(event EventBeginPlay
  (Utilities|Time|SetTimerbyEvent 0 (Variables|Default|GetSpawnDuration))
  (bind _returnvalue (Class|ProjectileSpawner|GetNearbyEnemies))
  (bind _output_get (Variables|Default|SetPeriod (/ (Variables|Default|GetSpawnDuration) (Variables|Default|GetNumProjectiles))))
  (bind _returnvalue_2 (Utilities|Time|SetTimerbyEvent (delegate Custom|ProjectileSpawn) _output_get true))
  (Variables|Default|SetProjectileSpawnTimer _returnvalue_2))

(fn ConstructionScript)