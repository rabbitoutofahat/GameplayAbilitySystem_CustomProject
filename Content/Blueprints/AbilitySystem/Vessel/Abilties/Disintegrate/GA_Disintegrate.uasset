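; GA_Disintegrate is a gameplay ability that casts a projectile from the weapon socket toward the point under the mouse.
; After committing, it gets cursor target data, stores the hit location and actor, and turns the avatar to face that point.
; It plays a FireBolt cast montage, waits for the FireBolt montage event to spawn the projectile, then ends.
; Despite the Disintegrate name, montage and event are both FireBolt's.
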(event Ability|EventActivateAbility
  (Ability|CommitAbility)
  (bind _datahandle (|GetTargetDataUnderMouse)
    (:ValidData
      (Variables|Default|SetProjectileTargetLocation (.Location (Collision|BreakHitResult (Ability|TargetData|GetHitResultfromTargetData _datahandle))))
      (Variables|Default|SetMouseHitActor (.HitActor (Collision|BreakHitResult (Ability|TargetData|GetHitResultfromTargetData _datahandle))))
      (bind _returnvalue (Class|CombatInterface|GetCombatSocketLocation(Message) (Ability|GetAvatarActorfromActorInfo) (GameplayTags|MakeLiteralGameplayTag "(TagName=\"CombatSocket.Weapon\")")))
      (Variables|Default|SetCombatSocketLocation _returnvalue)
      (Class|CombatInterface|UpdateFacingTarget(Message) (Ability|GetAvatarActorfromActorInfo) (Variables|Default|GetProjectileTargetLocation))
      (|PlayMontageandWaitProxy "None" "/Game/Assets/Characters/Aura/Animations/Abilities/AM_Cast_FireBolt_2.AM_Cast_FireBolt_2" 1.0 "None" false 1.0 0.0 false
        (:then
          (Ability|Tasks|WaitGameplayEvent "(TagName=\"Event.Montage.FireBolt\")" 0
            (:EventReceived
              (Class|AuraProjectileSpell|SpawnProjectileatSocket (Variables|Default|GetProjectileTargetLocation) (GameplayTags|MakeLiteralGameplayTag "(TagName=\"CombatSocket.Weapon\")"))
              (Ability|EndAbility))))))))