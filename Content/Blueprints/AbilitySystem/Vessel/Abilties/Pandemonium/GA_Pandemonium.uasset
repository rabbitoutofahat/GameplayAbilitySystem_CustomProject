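; Vessel's Pandemonium gameplay ability, which empowers nearby summons by enabling their specials and applying a no-cost effect.
; On activation it gathers live players within a fixed radius around the avatar, intended to cover every summon, and casts each to SummonCharacter.
; Each summon applies the effect to its own ability system component.
; The ability commits only after the loop, ignoring the result, then ends immediately.
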(event Ability|EventActivateAbility
  (bind _output_get (Variables|Default|SetAvatarActor (Ability|GetAvatarActorfromActorInfo)))
  (bind _outoverlappingactors (Class|AuraAbilitySystemLibrary|GetLivePlayersWithinRadius _output_get (Utilities|Array|MakeArray _output_get) 1e+03 (Transformation|GetActorLocation _output_get))) ; Don't need to parameterise radius, always want to hit every summon so just set a really big number
  (for _array_element _outoverlappingactors
    (bind _assummon_character (Utilities|Casting|CastToSummonCharacter _array_element))
    (Class|SummonCharacter|ShouldEnableSpecial _assummon_character true)
    (GameplayEffects|ApplyGameplayEffectToSelf (Ability|GetAbilitySystemComponent _assummon_character) (Variables|Default|GetNoCostGameplayEffect) 1.0 (GameplayEffects|MakeEffectContext (Ability|GetAbilitySystemComponent _assummon_character))))
  (Ability|CommitAbility)
  (Ability|EndAbility))