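; BP_Meteor is a meteor projectile actor in the Summon Chaos Elemental ability's folder that rises or shifts vertically on spawn before launching.
; On BeginPlay a timeline adds its SpawnHeight value as a local Z offset on each update.
; The same update runs a three-second delay that then activates ProjectileMovement.
; Tick spins the actor on roll at a rate whose random range is collapsed to a constant.
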(event EventBeginPlay
  (Variables|Default|SetRollRotation%20Rate (Math|Random|RandomFloatinRange 1e+02 1e+02))
  (bind _spawnheight (Timeline|SpawnTimeline Play)
    (:Update
      (Transformation|AddActorLocalOffset (Math|Vector|MakeVector 0.0 0.0 _spawnheight) false false)
      (Utilities|FlowControl|Delay 3.0)
      (Components|Activation|Activate (Variables|Default|GetProjectileMovement) false))))

(event EventTick
  (params (DeltaSeconds :type Float%20%28single-precision%29))
  (Transformation|AddActorLocalRotation (Math|Rotator|MakeRotator (* DeltaSeconds (Variables|Default|GetRollRotation%20Rate)) 0.0 0.0) false false))

(fn ConstructionScript)