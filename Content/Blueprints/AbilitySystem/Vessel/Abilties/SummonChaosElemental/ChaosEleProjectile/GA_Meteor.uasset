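; GA_Meteor is a Gameplay Ability that casts a meteor volley at the avatar's combat target, apparently for the Chaos Elemental.
; It commits, turns the avatar toward the target, pre-spawns projectiles via SpawnProjectilesAboveActor using the target's location, then plays the cast montage.
; The Event.Montage.Meteor gameplay event activates each stored projectile's movement, syncing launch to the animation, and ends the ability.
; Montage interruption or cancellation ends the ability without launching them.
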(event Ability|EventActivateAbility
  (bind _returnvalue (Ability|GetAvatarActorfromActorInfo))
  (Ability|CommitAbility)
  (bind _returnvalue_2 (Class|CombatInterface|GetCombatTarget(Message) _returnvalue))
  (Class|CombatInterface|UpdateFacingTarget(Message) _returnvalue (Transformation|GetActorLocation _returnvalue_2))
  (bind _output_get (Variables|Default|SetProjectileTargetLocation (Transformation|GetActorLocation _returnvalue_2)))
  (bind _returnvalue_3 (Class|AuraProjectileSpell|SpawnProjectilesAboveActor _output_get (Variables|Default|GetMaxProjectiles) 2e+02))
  (Variables|Default|SetProjectiles _returnvalue_3)
  (|PlayMontageandWaitProxy "None" "/Game/Assets/Characters/ChaosElemental/Animations/Montages/AM_ChaosEle_Cast.AM_ChaosEle_Cast" 1.0 "None" true 1.0 0.0 false
    (:then
      (Ability|Tasks|WaitGameplayEvent "(TagName=\"Event.Montage.Meteor\")" 0
        (:EventReceived
          (for _array_element (Variables|Default|GetProjectiles)
            (Components|Activation|Activate (Variables|/Script/Aura.AuraProjectile|GetProjectileMovement _array_element) false))
          (Ability|EndAbility))))
    (:OnInterrupted
      (Ability|EndAbility :!label _label))
    (:OnCancelled
      (goto _label))))

(event Ability|EventOnEndAbility
  (params (bWasCancelled :type Boolean)))