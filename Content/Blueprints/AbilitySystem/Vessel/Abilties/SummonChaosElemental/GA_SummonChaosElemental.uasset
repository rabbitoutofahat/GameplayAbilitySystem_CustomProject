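; Gameplay ability for the Vessel that summons a Chaos Elemental beside the avatar.
; On activation it commits, then line-traces vertically on Visibility at a fixed world-space offset from the avatar to find ground.
; A hit passes a point raised above the impact, with the avatar's rotation, to SummonChaosElemental and ends the ability.
; A missed trace neither summons nor calls EndAbility.
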(event Ability|EventActivateAbility
  (Ability|CommitAbility)
  (bind _output_get (Variables|Default|SetAvatarActor (Ability|GetAvatarActorfromActorInfo)))
  (bind _outhit (Collision|LineTraceByChannel (+ (Transformation|GetActorLocation _output_get) "0.000000,150.000000,500.000000") (+ (Transformation|GetActorLocation _output_get) "0.000000,150.000000,-500.000000") "TraceTypeQuery1" false 0 "None"))
  (if (.bBlockingHit (Collision|BreakHitResult _outhit))
    (Class|SummonChaosElemental|SummonChaosElemental (Math|Transform|MakeTransform (+ (.ImpactPoint (Collision|BreakHitResult _outhit)) "0.000000,0.000000,88.000000") (Transformation|GetActorRotation (Variables|Default|GetAvatarActor)) "1.000000,1.000000,1.000000"))
    (Ability|EndAbility)))

(event Ability|EventOnEndAbility
  (params (bWasCancelled :type Boolean)))