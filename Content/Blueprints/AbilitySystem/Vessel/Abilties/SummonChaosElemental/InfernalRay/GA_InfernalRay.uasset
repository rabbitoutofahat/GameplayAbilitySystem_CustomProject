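; Gameplay ability for the Chaos Elemental summon's Infernal Ray, a channeled fire attack on its combat target.
; A montage event starts a looping cue from the weapon and a timer that repeatedly applies fire damage and grants the summon energy.
; The owning Vessel's Annihilation tag scales DamageEffectParams, though ticks read GetDamageAtLevel instead.
; Full energy, duration expiry, target death or montage interruption clears timers and cue, then ends the ability.
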(event Custom|DamageTick
  (if (Variables|/Script/Aura.SummonCharacter|GetbFullEnergy (stale Ability|EventActivateAbility _output_get_3))
    (CallFunction|PreparetoEndAbility)
    (Ability|EndAbility)
    (else
      (CallFunction|DealDamageandGenerateEnergy (Variables|Default|GetCombatTarget)))))

(event Custom|Duration
  (CallFunction|PreparetoEndAbility)
  (Ability|EndAbility))

(event Ability|EventActivateAbility
  (bind _returnvalue (Ability|GetAvatarActorfromActorInfo))
  (Ability|CommitAbility)
  (Variables|Default|SetAvatarActor _returnvalue)
  (bind _returnvalue_2 (Class|CombatInterface|GetCombatTarget(Message) _returnvalue))
  (bind _output_get (Variables|Default|SetCombatTarget _returnvalue_2))
  (Variables|Default|SetDamageEffectParams (Class|AuraDamageGameplayAbility|MakeDamageEffectParamsfromClassDefaults _output_get))
  (CallFunction|AnnihilationDamageIncrease)
  (Class|CombatInterface|UpdateFacingTarget(Message) (Variables|Default|GetAvatarActor) (Transformation|GetActorLocation _output_get))
  (Variables|Default|SetTargetLocation (Transformation|GetActorLocation _output_get))
  (|PlayMontageandWaitProxy "None" "/Game/Assets/Characters/ChaosElemental/Animations/Montages/AM_ChaosEle_InfernalRay.AM_ChaosEle_InfernalRay" 1.0 "None" true 1.0 0.0 false
    (:then
      (Ability|Tasks|WaitGameplayEvent "(TagName=\"Event.Montage.InfernalRay\")" 0 true
        (:EventReceived
          (bind _returnvalue_3 (Class|CombatInterface|GetWeapon(Message) (Variables|Default|GetAvatarActor)))
          (bind _output_get_2 (Variables|Default|SetCueParams (Ability|GameplayCue|MakeGameplayCueParameters :Location (Variables|Default|GetTargetLocation) :SourceObject (Variables|Default|GetCombatTarget) :TargetAttachComponent _returnvalue_3)))
          (GameplayCue|AddGameplayCueOnActor(Looping) (Variables|Default|GetCombatTarget) "(TagName=\"GameplayCue.ShockLoop.ChaosEle\")" _output_get_2)
          (bind _returnvalue_4 (Utilities|Time|SetTimerbyEvent (delegate Custom|Duration) (Variables|Default|GetAbilityDuration)))
          (Variables|Default|SetDurationTimer _returnvalue_4)
          (bind _assummon_character (Utilities|Casting|CastToSummonCharacter (Variables|Default|GetAvatarActor)))
          (bind _output_get_3 (Variables|Default|SetSummonCharacter _assummon_character))
          (bind _returnvalue_5 (Utilities|Time|SetTimerbyEvent (delegate Custom|DamageTick) (Variables|Default|GetDamageDeltaTime) true))
          (Variables|Default|SetDamageTimer _returnvalue_5))))
    (:OnInterrupted
      (CallFunction|PreparetoEndAbility :!label _label)
      (Ability|EndAbility))
    (:OnCancelled
      (goto _label))))

(event EventPrimaryTargetDied
  (params (DeadActor :type Actor%20Object%20Reference))
  ;[1 0.5395 0.1248] Primary Target Died -> Ability is done
  (CallFunction|PreparetoEndAbility)
  (Ability|EndAbility))

(fn DealDamageandGenerateEnergy
  (params (Target :type Actor%20Object%20Reference))
  (bind _output_get (LocalVariables|SetDamagedTarget Target))
  (Utilities|IsValid _output_get
    (:Is%20Valid
      (bind _output_get_2 (LocalVariables|SetASC (Ability|GetAbilitySystemComponentfromActorInfo)))
      (Utilities|IsValid _output_get_2
        (:Is%20Valid
          (bind _returnvalue (Ability|GameplayEffect|AssignTagSetbyCallerMagnitude (GameplayEffects|MakeOutgoingSpec (LocalVariables|GetASC) (Variables|Default|GetDamageEffectClass) (Math|Conversions|ToFloat(Integer) (Ability|GetAbilityLevel)) (GameplayEffects|MakeEffectContext (LocalVariables|GetASC))) "(TagName=\"Damage.Fire\")" (Class|AuraDamageGameplayAbility|GetDamageatLevel)))
          (Utilities|IsValid (Ability|GetAbilitySystemComponent (LocalVariables|GetDamagedTarget))
            (:Is%20Valid
              (GameplayEffects|ApplyGameplayEffectSpecToSelf (Ability|GetAbilitySystemComponent (LocalVariables|GetDamagedTarget)) _returnvalue)
              (CallFunction|GenerateEnergyonHit (Variables|Default|GetSummonCharacter)))))))))

(fn PreparetoEndAbility
  (Utilities|Time|ClearandInvalidateTimerbyHandle (Variables|Default|GetDamageTimer))
  (Utilities|Time|ClearandInvalidateTimerbyHandle (Variables|Default|GetDurationTimer))
  (GameplayCue|RemoveGameplayCueOnActor(Looping) (Variables|Default|GetCombatTarget) "(TagName=\"GameplayCue.ShockLoop.ChaosEle\")" (Variables|Default|GetCueParams))
  (Variables|Default|SetCombatTarget 0))

(fn GenerateEnergyonHit
  (params (SummonCharacter :type Summon%20Character%20Object%20Reference))
  (LocalVariables|SetAvatarASC (Ability|GetAbilitySystemComponent (Variables|Default|GetAvatarActor)))
  (bind _returnvalue (Class|CombatInterface|GetPlayerLevel(Message) (Variables|Default|GetAvatarActor)))
  (bind _returnvalue_2 (Ability|GameplayEffect|AssignTagSetbyCallerMagnitude (Ability|MakeOutgoingGameplayEffectSpec "/Game/Blueprints/AbilitySystem/Vessel/Effects/GE_EnergyRegen.GE_EnergyRegen_C" (Math|Conversions|ToFloat(Integer) _returnvalue)) (Variables|Default|GetEnergyTag) (Variables|/Script/Aura.SummonCharacter|GetEnergyOnHit SummonCharacter)))
  (GameplayEffects|ApplyGameplayEffectSpecToSelf (LocalVariables|GetAvatarASC) _returnvalue_2))

(fn AnnihilationDamageIncrease
  (bind _assummon_character (Utilities|Casting|CastToSummonCharacter (Variables|Default|GetAvatarActor)))
  (bind _asvessel (Utilities|Casting|CastToVessel (Variables|/Script/Aura.SummonCharacter|GetOwnerActor _assummon_character)))
  (bind _asaura_ability_system_component (Utilities|Casting|CastToAuraAbilitySystemComponent (Ability|GetAbilitySystemComponent _asvessel)))
  (bind _output_get (LocalVariables|SetVesselASC _asaura_ability_system_component))
  (if (GameplayTags|HasMatchingGameplayTag _output_get "(TagName=\"Abilities.Vessel.SummonChaosElemental.Annihilation\")")
    (bind _structout (Utilities|Struct|SetmembersinDamageEffectParams (Variables|Default|GetDamageEffectParams) (* (.basedamage (Variables|Default|GetDamageEffectParams)) (Variables|Default|GetAnnihilationDamageCoeff))))
    (Variables|Default|SetDamageEffectParams _structout)))