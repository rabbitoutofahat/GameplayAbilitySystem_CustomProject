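; GA_SummonDregling is a Vessel gameplay ability that launches a Dregling projectile at the point under the mouse.
; On activation it commits, then waits on a target-data-under-mouse task for a valid hit.
; It stores the hit location and actor, turns the avatar toward the location, spawns the projectile with X/Y offsets, and ends.
; Only the valid-data path ends the ability, and the commit result is not checked.
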(event Ability|EventActivateAbility
  (Ability|CommitAbility)
  (bind _datahandle (|GetTargetDataUnderMouse)
    (:ValidData
      (bind _output_get (Variables|Default|SetTargetLocation (.Location (Collision|BreakHitResult (Ability|TargetData|GetHitResultfromTargetData _datahandle)))))
      (Variables|Default|SetMouseHitActor (.HitActor (Collision|BreakHitResult (Ability|TargetData|GetHitResultfromTargetData _datahandle))))
      (Class|CombatInterface|UpdateFacingTarget(Message) (Ability|GetAvatarActorfromActorInfo) _output_get)
      (Class|SummonDregling|SpawnDreglingProjectile (Variables|Default|GetTargetLocation) (Variables|Default|GetXOffset) (Variables|Default|GetYOffset))
      (Ability|EndAbility))))