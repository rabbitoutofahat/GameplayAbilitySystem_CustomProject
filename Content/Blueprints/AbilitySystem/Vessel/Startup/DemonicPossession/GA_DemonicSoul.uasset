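; Gameplay ability for the Vessel character that summons a Demonic Soul minion for as long as the ability is active.
; On activation, a vertical visibility trace at a fixed world-space X offset from the avatar finds the ground.
; The soul spawns just above the hit, takes the owner's level and is stored on the Vessel.
; The graph never ends the ability itself; when it ends, the stored soul is destroyed.
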(event Ability|EventActivateAbility
  (bind _output_get (Variables|Default|SetAvatarActor (Ability|GetAvatarActorfromActorInfo)))
  (bind _outhit (Collision|LineTraceByChannel (+ (Transformation|GetActorLocation _output_get) "150.000000,0.000000,500.000000") (+ (Transformation|GetActorLocation _output_get) "150.000000,0.000000,-500.000000") "TraceTypeQuery1" false 0 "None"))
  (if (.bBlockingHit (Collision|BreakHitResult _outhit))
    (bind _asvessel (Utilities|Casting|CastToVessel (Variables|Default|GetAvatarActor)))
    (bind _output_get_2 (Variables|Default|SetVessel _asvessel))
    (bind _returnvalue (Class|CombatInterface|GetPlayerLevel(Message) _output_get_2))
    (bind _returnvalue_2 (Class|Vessel|SpawnSummonedMinion (Variables|Default|GetVessel) (Variables|/Script/Aura.Vessel|GetDemonicSoulClass (Variables|Default|GetVessel)) (Math|Transform|MakeTransform (+ (.ImpactPoint (Collision|BreakHitResult _outhit)) "0.000000,0.000000,88.000000") (Transformation|GetActorRotation (Variables|Default|GetAvatarActor)) "1.000000,1.000000,1.000000") _returnvalue))
    (bind _asdemonic_soul (Utilities|Casting|CastToDemonicSoul _returnvalue_2))
    (Variables|/Script/Aura.Vessel|SetDemonicSoul (Variables|Default|GetVessel) _asdemonic_soul)))

(event Ability|EventOnEndAbility
  (params (bWasCancelled :type Boolean))
  (bind _vessel (Variables|Default|GetVessel)
    (:then
      (bind _demonicsoul (Variables|/Script/Aura.Vessel|GetDemonicSoul _vessel)
        (:then
          (Actor|DestroyActor _demonicsoul))
        (:else)))
    (:else)))