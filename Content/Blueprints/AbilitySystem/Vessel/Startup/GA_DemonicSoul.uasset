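; Gameplay ability that summons a Demonic Soul minion beside the avatar and destroys it when the ability ends.
; On activation, a vertical Visibility trace at a fixed world-space offset from the avatar finds the ground.
; On a hit, the AuraCharacter spawns BP_DemonicSoul slightly above the impact point, passing the avatar's rotation and the player's level.
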(event Ability|EventActivateAbility
  (bind _output_get (Variables|Default|SetAvatarActor (Ability|GetAvatarActorfromActorInfo)))
  (bind _outhit (Collision|LineTraceByChannel (+ (Transformation|GetActorLocation _output_get) "150.000000,0.000000,500.000000") (+ (Transformation|GetActorLocation _output_get) "150.000000,0.000000,-500.000000") "TraceTypeQuery1" false 0 "None"))
  (if (.bBlockingHit (Collision|BreakHitResult _outhit))
    (bind _asaura_character (Utilities|Casting|CastToAuraCharacter (Variables|Default|GetAvatarActor)))
    (bind _returnvalue (Class|CombatInterface|GetPlayerLevel(Message) _asaura_character))
    (bind _returnvalue_2 (Class|AuraCharacter|SpawnSummonedMinion _asaura_character "/Game/Blueprints/Character/Vessel/DemonicSoul/BP_DemonicSoul.BP_DemonicSoul_C" (Math|Transform|MakeTransform (+ (.ImpactPoint (Collision|BreakHitResult _outhit)) "0.000000,0.000000,88.000000") (Transformation|GetActorRotation (Variables|Default|GetAvatarActor)) "1.000000,1.000000,1.000000") _returnvalue))
    (Variables|Default|SetDemonicSoul _returnvalue_2)))

(event Ability|EventOnEndAbility
  (params (bWasCancelled :type Boolean))
  (Actor|DestroyActor (Variables|Default|GetDemonicSoul)))