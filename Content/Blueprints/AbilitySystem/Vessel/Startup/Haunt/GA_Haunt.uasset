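; GA_Haunt is the Vessel's Haunt ability: it recalls the Demonic Soul with a return projectile, buffs both, then launches it back out.
; The passive effect lasts until input is pressed or the duration expires, then a montage event fires the soul at the mouse target.
; Ability tags add upgrades: stronger passive, health redistribution, or recall explosion plus buff.
; The ability commits only on firing, and ends early if the soul is dead or invalid.
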(event Ability|EventActivateAbility
  (bind _asvessel (Utilities|Casting|CastToVessel (Ability|GetAvatarActorfromActorInfo)))
  (bind _output_get (Variables|Default|SetVessel _asvessel))
  (Variables|Default|SetVesselASC (Ability|GetAbilitySystemComponent _output_get))
  (bind _output_get_2 (Variables|Default|SetDemonicSoul (Variables|/Script/Aura.Vessel|GetDemonicSoul _output_get)))
  (Utilities|IsValid _output_get_2
    (:Is%20Valid
      (bind _ascombat_interface (Utilities|Casting|CastToCombatInterface (Variables|Default|GetDemonicSoul)))
      (if (Class|CombatInterface|IsDead _ascombat_interface)
        (Ability|EndAbility)
        (else
          (if (GameplayTags|HasMatchingGameplayTag (Variables|Default|GetVesselASC) "(TagName=\"Abilities.Utility.Haunt.SoulInstability\")")
            (CallFunction|ExplodeonRecall))
          (Class|Haunt|SpawnReturnProjectile)
          (Utilities|FlowControl|Delay 1.0)
          (Audio|PlaySound2D (Variables|Default|GetReturnSound) 1.0 1.0 0.0 0 0)
          (CallFunction|ApplyHauntPassiveGameplayEffect)
          (Ability|Tasks|WaitInputPress false
            (:then
              (Utilities|FlowControl|Delay (Variables|Default|GetHauntDuration)))
            (:OnPress
              _))
          (CallFunction|RemoveHauntPassiveGameplayEffect)
          (bind _datahandle (|GetTargetDataUnderMouse)
            (:ValidData
              (Variables|Default|SetProjectileTargetLocation (.Location (Collision|BreakHitResult (Ability|TargetData|GetHitResultfromTargetData _datahandle))))
              (Variables|Default|SetMouseHitActor (.HitActor (Collision|BreakHitResult (Ability|TargetData|GetHitResultfromTargetData _datahandle))))
              (bind _returnvalue (Class|CombatInterface|GetCombatSocketLocation(Message) (Ability|GetAvatarActorfromActorInfo) (GameplayTags|MakeLiteralGameplayTag "(TagName=\"CombatSocket.Weapon\")")))
              (Variables|Default|SetCombatSocketLocation _returnvalue)
              (Class|CombatInterface|UpdateFacingTarget(Message) (Ability|GetAvatarActorfromActorInfo) (Variables|Default|GetProjectileTargetLocation))
              (|PlayMontageandWaitProxy "None" "/Game/Assets/Characters/Aura/Animations/Abilities/AM_Cast_FireBolt.AM_Cast_FireBolt" 1.0 "None" false 1.0 0.0 false
                (:then
                  (Ability|Tasks|WaitGameplayEvent "(TagName=\"Event.Montage.FireBolt\")" 0
                    (:EventReceived
                      (Class|Haunt|FireDemonicSoul (Variables|Default|GetProjectileTargetLocation) (GameplayTags|MakeLiteralGameplayTag "(TagName=\"CombatSocket.Weapon\")"))
                      (Ability|CommitAbility)
                      (Ability|EndAbility))))))))))
    (:Is%20Not%20Valid
      (Ability|EndAbility))))

(fn ApplyHauntPassiveGameplayEffect
  (bind _vesselasc (Variables|Default|GetVesselASC))
  (bind _vesselasc_2 (Variables|Default|GetVesselASC))
  (Variables|Default|SetPassiveEffectContext (GameplayEffects|MakeEffectContext _vesselasc))
  (if (GameplayTags|HasMatchingGameplayTag _vesselasc "(TagName=\"Abilities.Utility.Haunt.PerfectedForm\")")
    (bind _returnvalue (GameplayEffects|ApplyGameplayEffectToSelf (Variables|Default|GetVesselASC) (Variables|Default|GetUpgradedHauntPassiveEffectClass) 1.0 (Variables|Default|GetPassiveEffectContext)))
    (Variables|Default|SetVesselEffectHandle _returnvalue)
    (bind _output_get (Variables|Default|SetDemonicSoulASC (Ability|GetAbilitySystemComponent (Variables|Default|GetDemonicSoul))))
    (bind _returnvalue_2 (GameplayEffects|ApplyGameplayEffectToSelf _output_get (Variables|Default|GetUpgradedHauntPassiveEffectClass) 1.0 (Variables|Default|GetPassiveEffectContext)))
    (Variables|Default|SetDemonicSoulEffectHandle _returnvalue_2)
    (Variables|Default|SetHauntDuration 2e+01)
    (else
      (bind _returnvalue_3 (GameplayEffects|ApplyGameplayEffectToSelf (Variables|Default|GetVesselASC) (Variables|Default|GetHauntPassiveEffectClass) 0.0 (Variables|Default|GetPassiveEffectContext)))
      (Variables|Default|SetVesselEffectHandle _returnvalue_3)
      (bind _output_get_2 (Variables|Default|SetDemonicSoulASC (Ability|GetAbilitySystemComponent (Variables|Default|GetDemonicSoul))))
      (bind _returnvalue_4 (GameplayEffects|ApplyGameplayEffectToSelf _output_get_2 (Variables|Default|GetHauntPassiveEffectClass) 1.0 (Variables|Default|GetPassiveEffectContext)))
      (Variables|Default|SetDemonicSoulEffectHandle _returnvalue_4)))
  (Utilities|FlowControl|Sequence
    (:then_0
      ;[1 1 1] Binding Contract Upgrade
      (if (GameplayTags|HasMatchingGameplayTag (Variables|Default|GetVesselASC) "(TagName=\"Abilities.Utility.Haunt.BindingContract\")")
        (Class|AuraAbilitySystemLibrary|RedistributeHealthEvenly (Utilities|Array|MakeArray (Variables|Default|GetVessel) (Variables|Default|GetDemonicSoul)))))
    (:then_1
      ;[1 1 1] Soul Instability Upgrade
      (if (GameplayTags|HasMatchingGameplayTag (Variables|Default|GetVesselASC) "(TagName=\"Abilities.Utility.Haunt.SoulInstability\")")
        (GameplayEffects|ApplyGameplayEffectToSelf _vesselasc_2 "/Game/Blueprints/AbilitySystem/Vessel/Startup/Haunt/Upgrades/SoulInstability/GE_SoulInstabilityBuff.GE_SoulInstabilityBuff_C" 1.0 (GameplayEffects|MakeEffectContext _vesselasc_2))))))

(fn RemoveHauntPassiveGameplayEffect
  (GameplayEffects|RemoveActiveGameplayEffect (Variables|Default|GetVesselASC) (Variables|Default|GetVesselEffectHandle) -1)
  (GameplayEffects|RemoveActiveGameplayEffect (Variables|Default|GetDemonicSoulASC) (Variables|Default|GetDemonicSoulEffectHandle) -1))

(fn ExplodeonRecall
  (bind _output_get (LocalVariables|SetDamageEffectParams (Class|AuraDamageGameplayAbility|MakeDamageEffectParamsfromClassDefaults 0)))
  (bind _structout (Utilities|Struct|SetmembersinDamageEffectParams _output_get (Transformation|GetActorLocation (Variables|Default|GetDemonicSoul))))
  (bind _outoverlappingactors (Class|AuraAbilitySystemLibrary|GetLivePlayersWithinRadius (.worldcontextobject _structout) (Utilities|Array|MakeArray (Variables|Default|GetVessel)) (.radialdamageouterradius _structout) (.radialdamageorigin _structout)))
  (for _array_element _outoverlappingactors
    (Utilities|IsValid (Ability|GetAbilitySystemComponent _array_element)
      (:Is%20Valid
        (bind _structout_2 (Utilities|Struct|SetmembersinDamageEffectParams (LocalVariables|GetDamageEffectParams) (Ability|GetAbilitySystemComponent _array_element) (* (Transformation|GetActorForwardVector _array_element) (.deathimpulsemagnitude _structout))))
        (Class|AuraAbilitySystemLibrary|ApplyDamageEffecttoTarget _structout_2))))
  (Audio|PlaySoundatLocation "/Game/Assets/Sounds/Abilities/FireBolt/sfx_FireBolt_Impact.sfx_FireBolt_Impact" (.radialdamageorigin _structout) "0, 0, 0" 1.0 1.0 0.0 0 0 0 0)
  (Niagara|SpawnSystematLocation "/Game/Assets/Effects/Projectiles/FireExplosion/NS_HauntExplosion.NS_HauntExplosion" (.radialdamageorigin _structout)))