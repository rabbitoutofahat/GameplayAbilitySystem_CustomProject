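; Soul Siphon gameplay ability for the Vessel, cast on the enemy under the mouse; it ends immediately if the hit actor is not a BP_EnemyBase enemy.
; Turns the caster to the target, attaches a buildup effect to the enemy's stun debuff component and plays the cast montage.
; The montage's gameplay event triggers the inherited SoulSiphon call and impact effect, then ends the ability, as does montage interruption or cancellation.
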(event Ability|EventActivateAbility
  (Ability|CommitAbility)
  (bind _datahandle (|GetTargetDataUnderMouse)
    (:ValidData
      (Variables|Default|SetTargetLocation (.Location (Collision|BreakHitResult (Ability|TargetData|GetHitResultfromTargetData _datahandle))))
      (Variables|Default|SetMouseHitActor (.HitActor (Collision|BreakHitResult (Ability|TargetData|GetHitResultfromTargetData _datahandle))))
      (if (Utilities|DoesObjectImplementInterface (Variables|Default|GetMouseHitActor) "/Script/Aura.EnemyInterface")
        (Class|CombatInterface|UpdateFacingTarget(Message) (Ability|GetAvatarActorfromActorInfo) (Variables|Default|GetTargetLocation))
        (bind _asbp_enemy_base (Utilities|Casting|CastToBP_EnemyBase (Variables|Default|GetMouseHitActor))
          (:then
            (bind _output_get (Variables|Default|SetDebuffComponent (Class|AuraCharacterBase|GetStunDebuffComponent _asbp_enemy_base)))
            (Niagara|SpawnSystemAttached "/Game/Assets/Effects/Combat/NS_SoulSiphonBuildup.NS_SoulSiphonBuildup" _output_get "None" "0, 0, 0" "0, 0, 0" "KeepRelativeOffset" false)
            (|PlayMontageandWaitProxy "None" "/Game/Assets/Characters/Aura/Animations/Abilities/AM_Cast_SoulSiphon.AM_Cast_SoulSiphon" 1.0 "None" false 1.0 0.0 false
              (:then
                (Ability|Tasks|WaitGameplayEvent "(TagName=\"Event.Montage.SoulSiphon\")" 0
                  (:EventReceived
                    (Class|SoulSiphon|SoulSiphon (Variables|Default|GetMouseHitActor))
                    (Niagara|SpawnSystemAttached "/Game/Assets/Effects/Combat/NS_SoulSiphonImpact.NS_SoulSiphonImpact" (Variables|Default|GetDebuffComponent) "None" "0, 0, 0" "0, 0, 0" "KeepRelativeOffset" false)
                    (Ability|EndAbility))))
              (:OnInterrupted
                (Ability|EndAbility :!label _label))
              (:OnCancelled
                (goto _label))))
          (:CastFailed
            (Ability|EndAbility)))
        (else
          (Ability|EndAbility))))))