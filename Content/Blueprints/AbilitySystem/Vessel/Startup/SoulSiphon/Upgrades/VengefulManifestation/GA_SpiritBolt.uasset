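; GA_SpiritBolt is a gameplay ability, under the Vessel's Soul Siphon Vengeful Manifestation upgrade, that fires a projectile at the avatar's combat target.
; On activation it commits, turns the avatar toward the target and stores that target's location.
; It plays the Spirit Bolt montage, whose gameplay event triggers the spawn at the weapon socket toward the stored location.
; The ability ends after spawning or when the montage finishes or is interrupted.
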(event Ability|EventActivateAbility
  (bind _returnvalue (Ability|GetAvatarActorfromActorInfo))
  (Ability|CommitAbility)
  (Variables|Default|SetAvatarActor _returnvalue)
  (bind _returnvalue_2 (Class|CombatInterface|GetCombatTarget(Message) _returnvalue))
  (bind _output_get (Variables|Default|SetCombatTarget _returnvalue_2))
  (Class|CombatInterface|UpdateFacingTarget(Message) _returnvalue (Transformation|GetActorLocation _output_get))
  (Variables|Default|SetTargetLocation (Transformation|GetActorLocation _output_get))
  (|PlayMontageandWaitProxy "None" "/Game/Assets/Enemies/Shaman/Animations/AM_Attack_SpiritBolt.AM_Attack_SpiritBolt" 1.0 "None" false 1.0 0.0 false
    (:then
      (Ability|Tasks|WaitGameplayEvent "(TagName=\"Event.Montage.SpiritBolt\")" 0
        (:EventReceived
          (Class|AuraProjectileSpell|SpawnProjectileatSocket (Variables|Default|GetTargetLocation) (GameplayTags|MakeLiteralGameplayTag "(TagName=\"CombatSocket.Weapon\")"))
          (Ability|EndAbility))))
    (:OnCompleted
      (Ability|EndAbility :!label _label))
    (:OnBlendOut
      (goto _label))
    (:OnInterrupted
      (goto _label))
    (:OnCancelled
      (goto _label))))