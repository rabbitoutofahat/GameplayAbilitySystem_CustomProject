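; Gameplay ability for the Chaos Elemental summon's special attack, which spawns projectiles aimed at the combat target's location.
; On activation it faces the target, caches that location and plays a montage, spawning the projectiles when the montage's gameplay event arrives.
; Cost is settled after spawning: a buff tag makes it consume a Demonic Strength stack and commit only cooldown, otherwise it commits normally.
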(event Ability|EventActivateAbility
  (bind _returnvalue (Ability|GetAvatarActorfromActorInfo))
  (bind _output_get (Variables|Default|SetAvatarActor _returnvalue))
  (bind _returnvalue_2 (Class|CombatInterface|GetCombatTarget(Message) _output_get))
  (Class|CombatInterface|UpdateFacingTarget(Message) _returnvalue (Transformation|GetActorLocation _returnvalue_2))
  (Variables|Default|SetProjectileTargetLocation (Transformation|GetActorLocation _returnvalue_2))
  (|PlayMontageandWaitProxy "None" "/Game/Assets/Characters/ChaosElemental/Animations/Montages/AM_ChaosEle_SpecialAttack.AM_ChaosEle_SpecialAttack" 1.0 "None" true 1.0 0.0 false
    (:then
      (Ability|Tasks|WaitGameplayEvent "(TagName=\"Event.Montage.Special.ChaosElemental\")" 0
        (:EventReceived
          (Class|AuraProjectileSpell|SpawnProjectilesAboveActor (Variables|Default|GetProjectileTargetLocation) (Variables|Default|GetMaxProjectiles) 1.8e+02)
          (CallFunction|DetermineAbilityCost)
          (Ability|EndAbility))))
    (:OnInterrupted
      (Ability|EndAbility :!label _label))
    (:OnCancelled
      (goto _label))))

(fn DetermineAbilityCost
  (if (GameplayTags|HasMatchingGameplayTag (Ability|GetAbilitySystemComponent (Variables|Default|GetAvatarActor)) (LocalVariables|GetBuffTag))
    (Ability|RemoveGameplayEffectFromOwnerWithGrantedTags "(GameplayTags=((TagName=\"Buff.DemonicStrength\")))" 1)
    (Ability|CommitAbilityCooldown false)
    (else
      (Ability|CommitAbility))))