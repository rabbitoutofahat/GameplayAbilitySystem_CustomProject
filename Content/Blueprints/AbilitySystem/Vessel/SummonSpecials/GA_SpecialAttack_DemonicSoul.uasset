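; Demonic Soul summon's special attack ability, which damages enemies in a sphere ahead of it when a montage event fires.
; Upgrade tags on the owning Vessel boost damage through Uproar and Spatial Rend.
; Spatial Rend can also spawn a ground-traced Lesser Demon, which may proc Portent of Destruction on the Vessel.
; The buff tag switches the commit to cooldown only, consuming a Demonic Strength stack instead of paying cost.
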(event Ability|EventActivateAbility
  (bind _demonicsoul (Variables|Default|GetDemonicSoul))
  (CallFunction|SetVariables)
  (Variables|Default|SetHasSpatialRendUpgrade (GameplayTags|HasMatchingGameplayTag (Variables|Default|GetVesselASC) "(TagName=\"Abilities.Passive.DemonicSoul.SpatialRend\")"))
  (|PlayMontageandWaitProxy "None" "/Game/Assets/Characters/DemonicSoul/Animations/Montages/AM_DemonicSoul_Special.AM_DemonicSoul_Special" 1.0 "None" true 1.0 0.0 false
    (:then
      (Ability|Tasks|WaitGameplayEvent "(TagName=\"Event.Montage.Special.DemonicSoul\")" 0
        (:EventReceived
          (bind _outoverlappingactors (Class|AuraAbilitySystemLibrary|GetLivePlayersWithinRadius _demonicsoul (Utilities|Array|MakeArray _demonicsoul) (Variables|Default|GetAttackRadius) (CallFunction|CalculateSphereDistanceBasedonRadius _demonicsoul)))
          (for _array_element _outoverlappingactors
            (bind _output_get (Variables|Default|SetEnemyActor _array_element))
            (if (not (Class|AuraAbilitySystemLibrary|IsonSameTeam _array_element (Variables|Default|GetDemonicSoul)))
              (Variables|Default|SetDamageEffectParams (Class|AuraDamageGameplayAbility|MakeDamageEffectParamsfromClassDefaults _output_get))
              (CallFunction|UproarDamageIncrease)
              (if (Variables|Default|GetHasSpatialRendUpgrade)
                (CallFunction|SpatialRendDamageIncrease))
              (Class|AuraAbilitySystemLibrary|ApplyDamageEffecttoTarget (Variables|Default|GetDamageEffectParams))
              (bind _asbp_enemy_base (Utilities|Casting|CastToBP_EnemyBase (Variables|Default|GetEnemyActor)))
              (Niagara|SpawnSystemAttached "/Game/Assets/Effects/ManaDrain/NS_DemonicSoul_SpecialHit.NS_DemonicSoul_SpecialHit" (Class|AuraCharacterBase|GetStunDebuffComponent _asbp_enemy_base) "None" "0, 0, 0" "0, 0, 0" "KeepRelativeOffset" false)))
          (if (Variables|Default|GetHasSpatialRendUpgrade)
            (CallFunction|SpawnLesserDemon))
          (CallFunction|DetermineAbilityCost)
          (Ability|EndAbility))))
    (:OnInterrupted
      (Ability|EndAbility :!label _label))
    (:OnCancelled
      (goto _label))))

(fn CalculateSphereDistanceBasedonRadius
  (params (AvatorActor :type Actor%20Object%20Reference))
  (return (+ (Transformation|GetActorLocation AvatorActor) (* (Transformation|GetActorForwardVector AvatorActor) (Variables|Default|GetAttackRadius)))))

(fn DetermineAbilityCost
  (if (GameplayTags|HasMatchingGameplayTag (Ability|GetAbilitySystemComponent (Variables|Default|GetDemonicSoul)) (Variables|Default|GetBuffTag))
    (Ability|RemoveGameplayEffectFromOwnerWithGrantedTags "(GameplayTags=((TagName=\"Buff.DemonicStrength\")))" 1)
    (Ability|CommitAbilityCooldown false)
    (else
      (Ability|CommitAbility))))

(fn SpatialRendDamageIncrease
  (bind _structout (Utilities|Struct|SetmembersinDamageEffectParams (Variables|Default|GetDamageEffectParams) (* (.basedamage (Variables|Default|GetDamageEffectParams)) (Variables|/Script/Aura.DemonicSoul|GetDamageCoefficient (Variables|Default|GetDemonicSoul)))))
  (Variables|Default|SetDamageEffectParams _structout))

(fn SpawnLesserDemon
  (bind _demonicsoul (Variables|Default|GetDemonicSoul))
  (bind _vessel (Variables|Default|GetVessel))
  (bind _returnvalue (Transformation|GetActorLocation _demonicsoul))
  (if (<= (Math|Random|RandomFloat) (Variables|/Script/Aura.DemonicSoul|GetLesserDemonSpawnPercent (Variables|Default|GetDemonicSoul)))
    (bind _outhit (Collision|LineTraceByChannel (+ _returnvalue "0.000000,-150.000000,500.000000") (+ _returnvalue "0.000000,-150.000000,-500.000000") "TraceTypeQuery1" false 0 "None"))
    (if (.bBlockingHit (Collision|BreakHitResult _outhit))
      (bind _returnvalue_2 (Class|CombatInterface|GetPlayerLevel _vessel))
      (Class|Vessel|SpawnSummonedMinion _vessel (Variables|/Script/Aura.Vessel|GetLesserDemonClass _vessel) (Math|Transform|MakeTransform (+ (.ImpactPoint (Collision|BreakHitResult _outhit)) "0.000000,0.000000,88.000000") (Transformation|GetActorRotation (Variables|Default|GetDemonicSoul)) "1.000000,1.000000,1.000000") _returnvalue_2)
      (CallFunction|PortentOfDestructionProc))))

(fn PortentOfDestructionProc
  (bind _vesselasc (Variables|Default|GetVesselASC))
  (if (GameplayTags|HasMatchingGameplayTag (Variables|Default|GetVesselASC) "(TagName=\"Abilities.Vessel.SummonDregling.PortentOfDestruction\")")
    (bind _returnvalue (Class|SummonDregling|GetPortentProcChance (Variables|Default|GetVesselASC)))
    (if (<= (Math|Random|RandomFloat) _returnvalue)
      (GameplayEffects|ApplyGameplayEffectToSelf _vesselasc "/Game/Blueprints/AbilitySystem/Vessel/Abilties/SummonDregling/Upgrades/PortentOfDestruction/GE_PortentOfDestructionBuff.GE_PortentOfDestructionBuff_C" 0.0 (GameplayEffects|MakeEffectContext _vesselasc)))))

(fn SetVariables
  (bind _asdemonic_soul (Utilities|Casting|CastToDemonicSoul (Ability|GetAvatarActorfromActorInfo)))
  (bind _output_get (Variables|Default|SetDemonicSoul _asdemonic_soul))
  (bind _asvessel (Utilities|Casting|CastToVessel (Variables|/Script/Aura.SummonCharacter|GetOwnerActor _output_get)))
  (bind _output_get_2 (Variables|Default|SetVessel _asvessel))
  (bind _asaura_ability_system_component (Utilities|Casting|CastToAuraAbilitySystemComponent (Ability|GetAbilitySystemComponent _output_get_2)))
  (Variables|Default|SetVesselASC _asaura_ability_system_component))

(fn UproarDamageIncrease
  (if (and (GameplayTags|HasMatchingGameplayTag (Variables|Default|GetVesselASC) "(TagName=\"Abilities.Vessel.Pandemonium.Uproar\")") (GameplayTags|HasMatchingGameplayTag (Ability|GetAbilitySystemComponent (Variables|Default|GetDemonicSoul)) "(TagName=\"Buff.DemonicStrength\")"))
    (bind _structout (Utilities|Struct|SetmembersinDamageEffectParams (Variables|Default|GetDamageEffectParams) (* (.basedamage (Variables|Default|GetDamageEffectParams)) (Variables|/Script/Aura.SummonCharacter|GetUproarDamageCoeff (Variables|Default|GetDemonicSoul)))))
    (Variables|Default|SetDamageEffectParams _structout)))