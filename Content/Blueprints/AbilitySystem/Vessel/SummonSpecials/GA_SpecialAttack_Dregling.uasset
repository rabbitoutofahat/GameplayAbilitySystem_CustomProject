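; Gameplay ability for the Dregling summon's special attack, a self-destruct that ends in an explosion.
; On activation it settles cost, starts the death montage and dissolve without waiting for the montage to finish, then explodes after a timer and ends.
; If the avatar has the buff tag, it removes one Demonic Strength stack and commits only the cooldown, otherwise it commits the full ability.
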(event Ability|EventActivateAbility
  (CallFunction|DetermineAbilityCost)
  (|PlayMontageandWaitProxy "None" "/Game/Assets/Characters/Dregling/Animations/Montages/AM_Dregling_Death.AM_Dregling_Death" 1.0 "None" true 1.0 0.0 false
    (:then
      (Class|DreglingExplosion|StartDissolve)
      (Utilities|FlowControl|Delay (Variables|Default|GetExplosionTimer))
      (Class|DreglingExplosion|Explosion)
      (Ability|EndAbility))))

(fn DetermineAbilityCost
  (if (GameplayTags|HasMatchingGameplayTag (Ability|GetAbilitySystemComponent (Ability|GetAvatarActorfromActorInfo)) (LocalVariables|GetBuffTag))
    (Ability|RemoveGameplayEffectFromOwnerWithGrantedTags "(GameplayTags=((TagName=\"Buff.DemonicStrength\")))" 1)
    (Ability|CommitAbilityCooldown false)
    (else
      (Ability|CommitAbility))))