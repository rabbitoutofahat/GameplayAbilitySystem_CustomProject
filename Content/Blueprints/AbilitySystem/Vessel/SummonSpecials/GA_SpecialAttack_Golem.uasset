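; Gameplay ability for the Infernal Golem summon's special attack, a radial slam.
; Plays a montage, then on its gameplay event fires the Upheaval cue and damages enemies in radius with upward knockback.
; Damage scales up when the golem has Demonic Strength and its owner has the Uproar ability tag.
; After the hit, a buffed golem spends a Demonic Strength stack and commits only cooldown; otherwise the ability commits normally.
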(event Ability|EventActivateAbility
  (bind _assummon_character (Utilities|Casting|CastToSummonCharacter (Ability|GetAvatarActorfromActorInfo)))
  (Variables|Default|SetAvatarActor _assummon_character)
  (|PlayMontageandWaitProxy "None" "/Game/Assets/Characters/InfernalGolem/Animations/Montages/AM_SpecialAttack_Golem.AM_SpecialAttack_Golem" 1.0 "None" true 1.0 0.0 false
    (:then
      (Ability|Tasks|WaitGameplayEvent "(TagName=\"Event.Montage.Special.InfernalGolem\")" 0
        (:EventReceived
          (GameplayCue|ExecuteGameplayCueOnActor(Burst) (Variables|Default|GetAvatarActor) "(TagName=\"GameplayCue.Upheaval\")" (Ability|GameplayCue|MakeGameplayCueParameters :Location (Transformation|GetActorLocation (Variables|Default|GetAvatarActor))))
          (CallFunction|ApplyRadialDamagetoAreaandEndAbility))))
    (:OnInterrupted
      (Ability|EndAbility :!label _label))
    (:OnCancelled
      (goto _label))))

(fn ApplyRadialDamagetoAreaandEndAbility
  (bind _avataractor (Variables|Default|GetAvatarActor))
  (bind _outoverlappingactors (Class|AuraAbilitySystemLibrary|GetLivePlayersWithinRadius _avataractor (Utilities|Array|MakeArray _avataractor) (Variables|Default|GetRadialDamageOuterRadius) (Transformation|GetActorLocation (Variables|Default|GetAvatarActor))))
  (for _array_element _outoverlappingactors
    (bind _output_get (Variables|Default|SetTargetActor _array_element))
    (if (not (Class|AuraAbilitySystemLibrary|IsonSameTeam _output_get (Variables|Default|GetAvatarActor)))
      (bind _structout (Utilities|Struct|SetmembersinDamageEffectParams (Class|AuraDamageGameplayAbility|MakeDamageEffectParamsfromClassDefaults (Variables|Default|GetTargetActor)) (CallFunction|DeathImpulse) (CallFunction|KnockbackImpulse) (Transformation|GetActorLocation (Variables|Default|GetAvatarActor))))
      (Variables|Default|SetDamageEffectParams _structout)
      (CallFunction|UproarDamageIncrease)
      (Class|AuraAbilitySystemLibrary|ApplyDamageEffecttoTarget (Variables|Default|GetDamageEffectParams))))
  (CallFunction|DetermineAbilityCost)
  (Ability|EndAbility))

(fn DetermineAbilityCost
  (if (GameplayTags|HasMatchingGameplayTag (Ability|GetAbilitySystemComponent (Variables|Default|GetAvatarActor)) (LocalVariables|GetBuffTag))
    (Ability|RemoveGameplayEffectFromOwnerWithGrantedTags "(GameplayTags=((TagName=\"Buff.DemonicStrength\")))" 1)
    (Ability|CommitAbilityCooldown false)
    (else
      (Ability|CommitAbility))))

(fn DeathImpulse
  (return (* (Transformation|GetActorForwardVector (Variables|Default|GetAvatarActor)) (Variables|Default|GetDeathImpulseMagnitude))))

(fn KnockbackImpulse
  (return (* (Class|AuraDamageGameplayAbility|GetImpulse (Variables|Default|GetTargetActor) (Math|Vector|VectorUp) true 9e+01) (Variables|Default|GetKnockbackMagnitude))))

(fn UproarDamageIncrease
  (bind _avataractor (Variables|Default|GetAvatarActor))
  (if (and (GameplayTags|HasMatchingGameplayTag (Ability|GetAbilitySystemComponent _avataractor) "(TagName=\"Buff.DemonicStrength\")") (GameplayTags|HasMatchingGameplayTag (Ability|GetAbilitySystemComponent (Variables|/Script/Aura.SummonCharacter|GetOwnerActor _avataractor)) "(TagName=\"Abilities.Vessel.Pandemonium.Uproar\")"))
    (bind _structout (Utilities|Struct|SetmembersinDamageEffectParams (Variables|Default|GetDamageEffectParams) (* (.basedamage (Variables|Default|GetDamageEffectParams)) (Variables|/Script/Aura.SummonCharacter|GetUproarDamageCoeff _avataractor))))
    (Variables|Default|SetDamageEffectParams _structout)))